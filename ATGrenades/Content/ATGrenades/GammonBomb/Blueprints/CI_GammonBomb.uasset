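; Carryable Gammon bomb item that the player arms, then turns into a live grenade when dropped outside the inventory.
; Use arms it on the server with a cap-opening sound, and the Armed RepNotify swaps the mesh.
; Pickup records the owning pawn; an armed drop has the server spawn Grenade_GammonBomb with the item's transform and velocity, then destroy the item.
; An unconnected debug chain remains in the event graph.
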(event `PlaySoundFX`
  (`GameplayStatics.PlaySoundAtLocation` "/Game/ATGrenades/Common/Sound/Cap_Open.Cap_Open" (`self.K2_GetActorLocation`) (struct) 1.0 1.0 0.0 "/Game/ATGrenades/Common/Sound/A_Grenade.A_Grenade" null null))

(event `self.OnDrop`
  (bind _returnvalue (`self.GetItemState`))
  (if (`|EnumEquality` _returnvalue "InInventory")
    _
    (elif (`self.Armed`)
      (`KismetSystemLibrary.Delay` 0.05)
      (`self.OnDrop_Server` (`self.GetTransform`) (`self.GetVelocity`) (`self.OwnerPawn`)))))

(event `OnDrop_Server`
  (params (SpawnTransform :type "Transform Structure") (Velocity :type "Vector Structure") (Instigator :type "Pawn Object Reference"))
  (`|SpawnActorFromClass` "/Game/ATGrenades/GammonBomb/Blueprints/Grenade_GammonBomb.Grenade_GammonBomb_C" SpawnTransform "AlwaysSpawn" "OverrideRootScale" (`self.OwnerPawn`) Velocity (`self.Armed`) Instigator)
  (`KismetSystemLibrary.Delay` 0.2)
  (`self.K2_DestroyActor`))

(event `OnPickUp_Server`
  (params (OwnerPawn :type "Pawn Object Reference"))
  (set `self.OwnerPawn` OwnerPawn))

(event `self.OnPickup`
  (params (Pawn :type "Pawn Object Reference") (bDominant :type Boolean))
  (`self.OnPickUp_Server` Pawn))

(event `self.OnUse`
  (if (not (`self.Armed`))
    (`self.OnUse_Server`)))

(event `OnUse_Server`
  (set `self.Armed` true)
  (`self.PlaySoundFX`))

(fn `OnRep_Armed`
  (if (`self.Armed`)
    (`StaticMeshComponent.SetStaticMesh` (`self.Mesh`) "/Game/ATGrenades/GammonBomb/Meshes/GammonBomb.GammonBomb")))

(fn `UserConstructionScript`)