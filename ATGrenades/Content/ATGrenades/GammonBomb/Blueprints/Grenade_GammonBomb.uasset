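; Gammon bomb grenade projectile that launches at twice its Velocity value, explodes on impact when armed, and expires after 30 seconds.
; On a mesh hit, the server applies one radial falloff damage burst sized by two sphere components, plus direct damage to the hit actor.
; It then multicasts explosion particles, near and distant sounds and a decal attached to the hit component, and destroys itself after a brief delay.
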(event `self.ReceiveBeginPlay`
  (set `MovementComponent.Velocity` (* (`self.Velocity`) 2.0) (`self.ProjectileMovement`))
  (`self.SetLifeSpan` 30.0))

(event `self.Mesh.OnComponentHit`
  (params (HitComponent :type "PrimitiveComponent Object Reference") (OtherActor :type "Actor Object Reference") (OtherComp :type "PrimitiveComponent Object Reference") (NormalImpulse :type "Vector Structure") (Hit :type "HitResult Structure (by ref)"))
  (bind (_bblockinghit _binitialoverlap _time _distance _location _impactpoint _normal _impactnormal _physmat _hitactor _hitcomponent) (`GameplayStatics.BreakHitResult` Hit))
  (bind _returnvalue (`self.GetInstigatorController`))
  (`/Engine/EditorBlueprintResources/ActorMacros.Switch Has Authority`
    (:`Authority`
      (if (`self.Armed`)
        (`/Engine/EditorBlueprintResources/StandardMacros.DoOnce` false
          (:`Completed`
            (bind _output_get (set `self.AttachedComp` _hitcomponent))
            (`GameplayStatics.ApplyRadialDamageWithFalloff` :`BaseDamage` 200.0 :`MinimumDamage` 50.0 :`Origin` (`self.K2_GetActorLocation`) :`DamageInnerRadius` (`SphereComponent.GetScaledSphereRadius` (`self.InnerRadius`)) :`DamageOuterRadius` (`SphereComponent.GetScaledSphereRadius` (`self.OuterRadius`)) :`DamageFalloff` 0.5 :`DamageCauser` self :`InstigatedByController` _returnvalue)
            (`GameplayStatics.ApplyDamage` _hitactor 500.0 _returnvalue self)
            (`self.FX_Multicast` _impactpoint _normal _output_get)
            (`KismetSystemLibrary.Delay` 0.1)
            (`self.K2_DestroyActor`)))))))

(event `FX_Multicast`
  (params (Location :type "Vector Structure") (Normal :type "Vector Structure") (AttachToComponent :type "SceneComponent Object Reference"))
  (`GameplayStatics.SpawnEmitterAtLocation` (`self.FireEmitter`) Location (struct) (2.0 2.0 2.0))
  (`GameplayStatics.PlaySoundAtLocation` (`self.BulletExplosion`) Location (struct) 1.0 1.0 0.0 null null null)
  (`GameplayStatics.SpawnDecalAttached` (`self.ExplosionDecal`) (`KismetMathLibrary.Conv_DoubleToVector` (`SphereComponent.GetScaledSphereRadius` (`self.OuterRadius`))) AttachToComponent "None" Location (`KismetMathLibrary.MakeRotFromX` Normal) "KeepRelativeOffset" 10.0)
  (`GameplayStatics.PlaySoundAtLocation` (`self.BulletDistantExplosion`) Location (struct) 1.0 1.0 0.0 null null null))

(fn `UserConstructionScript`)