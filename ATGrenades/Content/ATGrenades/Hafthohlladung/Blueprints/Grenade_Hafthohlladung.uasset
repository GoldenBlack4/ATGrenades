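; Hafthohlladung sticky anti-tank grenade that attaches to the component it hit and explodes after a delay.
; On BeginPlay the authority runs Explode once with the Hit result, attaching the grenade through ReplicateAttach.
; After ExplosionDelay it applies falloff radial damage sized by two sphere components, plus heavy direct damage to the hit actor.
; A multicast plays explosion particles with near and distant sounds before the actor destroys itself.
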(event `self.ReceiveBeginPlay`
  (`self.SetLifeSpan` (+ (`self.ExplosionDelay`) 2.0))
  (`/Engine/EditorBlueprintResources/ActorMacros.Switch Has Authority`
    (:`Authority`
      (`self.Explode` (`self.Hit`)))))

(event `Explode`
  (params (Hit :type "HitResult Structure (by ref)"))
  (bind (_bblockinghit _binitialoverlap _time _distance _location _impactpoint _normal _impactnormal _physmat _hitactor _hitcomponent) (`GameplayStatics.BreakHitResult` Hit))
  (`/Engine/EditorBlueprintResources/ActorMacros.Switch Has Authority`
    (:`Authority`
      (`/Engine/EditorBlueprintResources/StandardMacros.DoOnce` false
        (:`Completed`
          (`self.ReplicateAttach` _hitcomponent)
          (set `self.HitComp` _hitcomponent)
          (set `self.HitActor` _hitactor)
          (`KismetSystemLibrary.Delay` (`self.ExplosionDelay`))
          (`GameplayStatics.ApplyRadialDamageWithFalloff` :`BaseDamage` 500.0 :`MinimumDamage` 80.0 :`Origin` (`self.K2_GetActorLocation`) :`DamageInnerRadius` (`SphereComponent.GetScaledSphereRadius` (`self.InnerRadius`)) :`DamageOuterRadius` (`SphereComponent.GetScaledSphereRadius` (`self.OuterRadius`)) :`DamageFalloff` 0.5 :`DamageCauser` self :`InstigatedByController` (`self.GetInstigatorController`))
          (`GameplayStatics.ApplyDamage` (`self.HitActor`) 2000.0 (`self.GetInstigatorController`) self)
          (`self.FX_Multicast`)
          (`KismetSystemLibrary.Delay` 0.1)
          (`self.K2_DestroyActor`))))))

(event `ReplicateAttach`
  (params (Parent :type "SceneComponent Object Reference"))
  (`self.K2_AttachToComponent` Parent "None" "KeepWorld" "KeepWorld" "KeepWorld"))

(event `FX_Multicast`
  (bind _returnvalue (`self.K2_GetActorLocation`))
  (`GameplayStatics.SpawnEmitterAtLocation` (`self.FireEmitter`) _returnvalue (struct) (2.0 2.0 2.0))
  (`GameplayStatics.PlaySoundAtLocation` (`self.BulletExplosion`) _returnvalue (struct) 1.0 1.0 0.0 null null null)
  (`GameplayStatics.PlaySoundAtLocation` (`self.BulletDistantExplosion`) _returnvalue (struct) 1.0 1.0 0.0 null null null))

(fn `UserConstructionScript`)