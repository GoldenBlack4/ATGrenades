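; Inventory item for the Hafthohlladung anti-tank charge, which sticks to vehicles once armed and out of the inventory.
; Use arms it on the server with a cap sound, and the Armed RepNotify swaps the mesh.
; A looping timer traces along the item's down axis, identifying vehicles by display-name matching.
; On a match, it spawns the grenade actor aligned to the surface with the explosion delay, then destroys itself.
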(event `self.OnDrop`)

(event `PlaySoundFX`
  ;[1 1 1] Sounds
  (`GameplayStatics.PlaySoundAtLocation` "/Game/ATGrenades/Common/Sound/Cap_Open.Cap_Open" (`self.K2_GetActorLocation`) (struct) 1.0 1.0 0.0 "/Game/ATGrenades/Common/Sound/A_Grenade.A_Grenade" null null))

(event `Pickup_Server`
  (params (OwnerPawn :type "Pawn Object Reference"))
  (set `self.OwnerPawn` OwnerPawn))

(event `self.OnPickup`
  (params (Pawn :type "Pawn Object Reference") (bDominant :type Boolean))
  (`self.Pickup_Server` Pawn))

(event `HitSoundFX`
  ;[1 1 1] Sounds
  (`GameplayStatics.PlaySoundAtLocation` "/Game/ATGrenades/Common/Sound/MetalHit.MetalHit" (`self.K2_GetActorLocation`) (struct) 1.0 1.0 0.0 "/Game/ATGrenades/Common/Sound/A_Grenade.A_Grenade" null null))

(event `self.OnUse`
  (if (not (`self.Armed`))
    (`self.OnUse_Server`)))

(event `OnUse_Server`
  (set `self.Armed` true)
  (bind _returnvalue (`KismetSystemLibrary.K2_SetTimerDelegate` (delegate `LineTrace`) 0.05 true))
  (set `self.LineTraceTimer` _returnvalue)
  (`self.PlaySoundFX`))

(event `LineTrace`
  (bind _returnvalue (`self.K2_GetActorLocation`))
  (bind _ownerpawn (`self.OwnerPawn`))
  (bind _returnvalue_2 (`self.GetItemState`))
  (if (not (`|EnumEquality` _returnvalue_2 "InInventory"))
    (bind (_outhit _returnvalue_3) (`KismetSystemLibrary.LineTraceSingle` :`Start` _returnvalue :`End` (+ _returnvalue (* (`KismetMathLibrary.GetUpVector` (`self.K2_GetActorRotation`)) -50.0)) :`TraceChannel` "TraceTypeQuery1" :`DrawDebugType` "Persistent"))
    (if _returnvalue_3
      (bind (_bblockinghit _binitialoverlap _time _distance _location _impactpoint _normal _impactnormal _physmat _hitactor) (`GameplayStatics.BreakHitResult` _outhit))
      (bind _returnvalue_4 (`KismetSystemLibrary.GetDisplayName` _hitactor))
      (if (or (`KismetStringLibrary.StartsWith` _returnvalue_4 "Veh") (`KismetStringLibrary.StartsWith` _returnvalue_4 "BPC_") (`KismetStringLibrary.StartsWith` _returnvalue_4 "BPM_") (`KismetStringLibrary.StartsWith` _returnvalue_4 "Tank") (`KismetStringLibrary.Contains` _returnvalue_4 "atv"))
        (`KismetSystemLibrary.K2_ClearAndInvalidateTimerHandle` (`self.LineTraceTimer`))
        (`/Engine/EditorBlueprintResources/StandardMacros.DoOnce` false
          (:`Completed`
            (`|SpawnActorFromClass` "/Game/ATGrenades/Hafthohlladung/Blueprints/Grenade_Hafthohlladung.Grenade_Hafthohlladung_C" (`KismetMathLibrary.MakeTransform` _location (`KismetMathLibrary.MakeRotFromZ` _impactnormal)) "AlwaysSpawn" "OverrideRootScale" _ownerpawn _outhit (`self.ExplosionDelay`) _ownerpawn)
            (`self.HitSoundFX`)
            (`KismetSystemLibrary.Delay` 0.1)
            (`self.K2_DestroyActor`)))))))

(fn `OnRep_Armed`
  (if (`self.Armed`)
    (`StaticMeshComponent.SetStaticMesh` (`self.Mesh`) "/Game/ATGrenades/Hafthohlladung/Meshes/hafthohlladung.hafthohlladung")))

(fn `UserConstructionScript`)